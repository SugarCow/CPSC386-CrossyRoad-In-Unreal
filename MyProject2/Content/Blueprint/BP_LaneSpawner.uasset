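; Lane spawner actor that creates randomly chosen road, river, field or train lanes.
; BeginPlay calls SpawnLane at a fixed location, which picks one of the four lane classes at random and stores the actor as NewestLane.
; SpawnLaneAtSpawnPoint spawns another at NewestLane's root location but is not called within this Blueprint.
; SpawnInitialLane's loop and the road-lane check after spawning are empty stubs.
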(event EventBeginPlay
  (CallFunction|SpawnLane "2000.000000, 0,500.000000"))

(event Collision|EventActorBeginOverlap
  (params (OtherActor :type Actor%20Object%20Reference)))

(event EventTick
  (params (DeltaSeconds :type Float%20%28single-precision%29)))

(fn ConstructionScript)

(fn SpawnLane
  (params (SpawnLocation :type Vector))
  (bind _returnvalue (Game|SpawnActorfromClass (Utilities|Select :Index (Math|Random|RandomIntegerinRange 0 3) :Option%200 "/Game/Blueprint/BP_Road_Lane.BP_Road_Lane_C" :Option%201 "/Game/Blueprint/BP_river_lane.BP_river_lane_C" :Option%202 "/Game/Blueprint/BP_Field_Lane.BP_Field_Lane_C" :Option%203 "/Game/Blueprint/BP_train_lane.BP_train_lane_C") (Math|Transform|MakeTransform SpawnLocation "0, 0, 0" "1.000000,1.000000,1.000000") "Undefined" 0 0))
  (bind _output_get (Variables|Default|SetNewestLane _returnvalue))
  (if (== _output_get "/Game/Blueprint/BP_Road_Lane.BP_Road_Lane")
    _))

(fn SpawnInitialLane
  (for _index (range 0 3)
    _))

(fn SpawnLaneatSpawnPoint
  (CallFunction|SpawnLane (Transformation|GetWorldLocation (Variables|/Script/Engine.Actor|GetRootComponent (Variables|Default|GetNewestLane)))))