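; BP_Field_Lane is a field lane that randomly scatters tree/rock spawners along its length when play begins.
; BeginPlay checks and flips LightGreen, switching the mesh to Field_type2 when the flag was false.
; It derives a slot count from the Start-to-End distance, then gives each slot a roughly one-in-five chance to spawn BP_Tree_rock_spawner.
; Slots step along world X from Start, at slightly wider spacing than the count assumes.
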(event EventBeginPlay
  (if (Variables|Default|GetLightGreen)
    (Variables|Default|SetLightGreen false)
    (else
      (Components|StaticMesh|SetStaticMesh (Variables|Default|GetStaticMesh) "/Game/blender_export/field_type2.field_type2")
      (Variables|Default|SetLightGreen true)))
  (bind _output_get (Variables|Default|SetStartLocation (Transformation|GetWorldLocation (Variables|Default|Getstart))))
  (bind _output_get_2 (Variables|Default|SetEndLocation (Transformation|GetWorldLocation (Variables|Default|Getend))))
  (for _index (range 0 (Math|Float|Truncate (/ (Math|Vector|Distance(Vector) _output_get _output_get_2) 85.0)))
    (if (> (Math|Random|RandomFloat) 0.8)
      (Game|SpawnActorfromClass "/Game/Blueprint/BP_Tree_rock_spawner.BP_Tree_rock_spawner_C" (Math|Transform|MakeTransform (Math|Vector|MakeVector (+ (.X (Math|Vector|BreakVector (Variables|Default|GetStartLocation))) (* _index 9e+01)) (.y (Variables|Default|GetStartLocation)) (.z (Variables|Default|GetStartLocation))) "0, 0, 0" "1.000000,1.000000,1.000000") "Undefined" 0 0))))

(fn ConstructionScript)