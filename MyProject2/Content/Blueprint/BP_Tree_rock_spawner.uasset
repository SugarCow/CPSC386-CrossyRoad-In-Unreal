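; BP_Tree_rock_spawner is a scenery Blueprint that randomizes whether it appears as a tree or a rock.
; On BeginPlay it rolls a random integer and switches on it to swap the StaticMesh component's mesh among tree and rock variants.
; A roll of zero has no case, so the component keeps its default mesh.
; The choice happens at runtime, as the construction script is empty.
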(event EventBeginPlay
  (switch int (Math|Random|RandomIntegerinRange 0 6)
    (:1
      (Components|StaticMesh|SetStaticMesh (Variables|Default|GetStaticMesh) "/Game/blender_export/tree_type2.tree_type2"))
    (:2
      (Components|StaticMesh|SetStaticMesh (Variables|Default|GetStaticMesh) "/Game/blender_export/tree_type1_tall.tree_type1_tall"))
    (:3
      (Components|StaticMesh|SetStaticMesh (Variables|Default|GetStaticMesh) "/Game/blender_export/tree_type2_tall.tree_type2_tall"))
    (:4
      (Components|StaticMesh|SetStaticMesh (Variables|Default|GetStaticMesh) "/Game/blender_export/rock_type1.rock_type1"))
    (:5
      (Components|StaticMesh|SetStaticMesh (Variables|Default|GetStaticMesh) "/Game/blender_export/rock_type2.rock_type2"))
    (:6
      (Components|StaticMesh|SetStaticMesh (Variables|Default|GetStaticMesh) "/Game/blender_export/rock_type2_1.rock_type2_1"))))

(fn ConstructionScript)